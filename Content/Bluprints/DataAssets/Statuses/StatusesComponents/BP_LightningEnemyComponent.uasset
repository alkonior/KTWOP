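; Lightning status component for enemies that reacts when the owner's LightningDMG status explodes.
; On BeginPlay it caches the owning BaseEnemy, then polls that status every Tick.
; The first time the status reports exploded, it calls the enemy's LightningBlastMessage and plays a bolt sound at its location.
; It destroys itself when the enemy dies or the status lookup fails.
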(event EventBeginPlay
  (bind _asbase_enemy (Utilities|Casting|CastToBaseEnemy (Components|GetOwner)))
  (Variables|Default|SetEnemy _asbase_enemy))

(event EventTick
  (params (DeltaSeconds :type Float%20%28single-precision%29))
  (bind _returnvalue (Class|StatusOwner|IsDead (Variables|Default|GetEnemy)))
  (if (not _returnvalue)
    (bind _returnvalue_2 (Class|StatusOwner|GetStatus(Message) (Variables|Default|GetEnemy) "LightningDMG"))
    (bind _aslightning_dmg (Utilities|Casting|CastToLightningDMG _returnvalue_2)
      (:then
        (if (Variables|/Script/ImplementedStatuses.ExplodedStatus|GetIsExploded _aslightning_dmg)
          (Utilities|FlowControl|DoOnce false
            (:Completed
              (Class|BPIEnemy|LightningBlast(Message) (Variables|Default|GetEnemy))
              (Audio|PlaySoundatLocation "/Game/Sounds/FireBolt/Cues/Fire_Bolts/Fire_bolt_2_Cue.Fire_bolt_2_Cue" (Transformation|GetActorLocation (Variables|Default|GetEnemy)) "0, 0, 0" 1.0 1.0 0.0 0 0 0 0)))))
      (:CastFailed
        (Components|DestroyComponent :!label _label)))
    (else
      (goto _label))))