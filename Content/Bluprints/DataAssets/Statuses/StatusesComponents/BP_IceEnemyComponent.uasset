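; Actor component for an enemy's ice status that keeps its ice message in sync with that status.
; It caches the owning BaseEnemy on begin play, then polls its IceDMG status message every tick and passes the IsExploded flag to SwitchIceMessage.
; When the enemy is dead or the status message is not a valid IceDMG, it switches the message off and destroys itself.
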(event EventBeginPlay
  (bind _asbase_enemy (Utilities|Casting|CastToBaseEnemy (Components|GetOwner)))
  (Variables|Default|SetEnemy _asbase_enemy))

(event EventTick
  (params (DeltaSeconds :type Float%20%28single-precision%29))
  (bind _returnvalue (Class|StatusOwner|IsDead (Variables|Default|GetEnemy)))
  (if (not _returnvalue)
    (bind _returnvalue_2 (Class|StatusOwner|GetStatus(Message) (Variables|Default|GetEnemy) "IceDMG"))
    (bind _asice_dmg (Utilities|Casting|CastToIceDMG _returnvalue_2)
      (:then
        (Class|BPIEnemy|SwitchIce(Message) (Variables|Default|GetEnemy) (Variables|/Script/ImplementedStatuses.ExplodedStatus|GetIsExploded _asice_dmg)))
      (:CastFailed
        (Class|BPIEnemy|SwitchIce(Message) (Variables|Default|GetEnemy) false :!label _label)
        (Components|DestroyComponent)))
    (else
      (goto _label))))