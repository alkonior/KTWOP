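; BP_CannonBuilding is a cannon building actor that shows or hides its static mesh according to its upgrade level.
; Its SetUpgradeLevel override hides the mesh at level 0, shows it at levels 1 to 3, and leaves visibility unchanged otherwise.
; Every branch then calls the parent implementation, and the event graph and construction script add no logic of their own.
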(event EventBeginPlay
  (|CallParentFunction) ; This node is disabled and will not be called.\nDrag off pins to build functionality.
)

(event Collision|EventActorBeginOverlap
  (params (OtherActor :type Actor%20Object%20Reference))
  (|CallParentFunction OtherActor) ; This node is disabled and will not be called.\nDrag off pins to build functionality.
)

(event EventTick
  (params (DeltaSeconds :type Float%20%28single-precision%29))
  (|CallParentFunction DeltaSeconds) ; This node is disabled and will not be called.\nDrag off pins to build functionality.
)

(fn ConstructionScript
  (|CallParentFunction))

(fn SetUpgradeLevel
  (params (NewLevel :type Integer))
  (switch int NewLevel
    (:Default
      (|CallParentFunction NewLevel))
    (:0
      (Rendering|SetVisibility (Variables|Default|GetStaticMesh) false false)
      (|CallParentFunction NewLevel))
    (:1
      (Rendering|SetVisibility (Variables|Default|GetStaticMesh) true false)
      (|CallParentFunction NewLevel))
    (:2
      (Rendering|SetVisibility (Variables|Default|GetStaticMesh) true false)
      (|CallParentFunction NewLevel))
    (:3
      (Rendering|SetVisibility (Variables|Default|GetStaticMesh) true false)
      (|CallParentFunction NewLevel))))