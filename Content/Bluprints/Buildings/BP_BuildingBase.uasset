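; BP_BuildingBase is a building Blueprint, apparently a base class, that manages the upgrade level of one building type.
; Levels are saved to the game instance's BuildingsLevels map keyed by Type, and Refresh reloads from it.
; Upgrade raises the level up to MaxLevel, otherwise printing a message.
; GetInfo looks up the type's row in DT_UI_BuildingInfo and returns the current level's data.
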(event EventBeginPlay)

(event Collision|EventActorBeginOverlap
  (params (OtherActor :type Actor%20Object%20Reference)))

(event EventTick
  (params (DeltaSeconds :type Float%20%28single-precision%29)))

(fn ConstructionScript)

(fn Refresh
  (CallFunction|SetUpgradeLevel (.Value (Utilities|Map|Find (Variables|/Game/Bluprints/Enemies/BP_KTWOPGameInstance.BP_KTWOPGameInstance_C|GetBuildingsLevels (.AsBP%20KTWOPGame%20Instance (Utilities|Casting|CastToBP_KTWOPGameInstance (Game|GetGameInstance)))) (Variables|Default|GetType)))))

(fn GetInfo
  (bind _returnvalue (Utilities|GetDataTableRow "/Game/UI/DT_UI_BuildingInfo.DT_UI_BuildingInfo" (Utilities|String|StringToName (Utilities|String|EnumtoString (Variables|Default|GetType))))
    (:then
      (return (|Copy (Utilities|Array|Get(acopy) (.buildingdataperlevel _returnvalue) (Variables|Default|GetLevel)))))))

(fn GetUpgradeLevlel
  (return (Variables|Default|GetLevel)))

(fn SetUpgradeLevel
  (params (NewLevel :type Integer))
  (bind _output_get (Variables|Default|SetLevel NewLevel))
  (Utilities|Map|Add (Variables|/Game/Bluprints/Enemies/BP_KTWOPGameInstance.BP_KTWOPGameInstance_C|GetBuildingsLevels (.AsBP%20KTWOPGame%20Instance (Utilities|Casting|CastToBP_KTWOPGameInstance (Game|GetGameInstance)))) (Variables|Default|GetType) _output_get))

(fn Upgrade
  (bind _level (Variables|Default|GetLevel))
  (bind _returnvalue (+ _level 1))
  (if (<= _returnvalue (Variables|Default|GetMaxLevel))
    (CallFunction|SetUpgradeLevel _returnvalue)
    (else
      (Development|PrintString "Can't upgrade anymore!!!"))))