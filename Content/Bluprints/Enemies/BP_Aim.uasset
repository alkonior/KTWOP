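; BP_Aim is the objective enemies attack: it holds HP shown on a widget bar and decides whether the level is won or lost.
; Enemies entering its sphere deal their AimDamage, are removed and count as defeated unless HP runs out, which fades out and opens L_World.
; Reaching the EnemiesCount total updates level states, saves and returns to L_World.
; The construction script snaps Point to the socket of the tile beneath.
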(event OnComponentBeginOverlap(Sphere)
  (params (OverlappedComponent :type Primitive%20Component%20Object%20Reference) (OtherActor :type Actor%20Object%20Reference) (OtherComp :type Primitive%20Component%20Object%20Reference) (OtherBodyIndex :type Integer) (bFromSweep :type Boolean) (SweepResult :type Hit%20Result%20Structure%20%28by%20ref%29))
  (bind _asbp_base_enemy (Utilities|Casting|CastToBP_BaseEnemy OtherActor))
  (bind _output_get (Variables|Default|SetHP (- (Variables|Default|GetHP) (Variables|/Game/Bluprints/Enemies/BP_BaseEnemy.BP_BaseEnemy_C|Getaim_damage _asbp_base_enemy))))
  (Development|PrintString (Utilities|String|ToString(Integer) _output_get))
  (Default|HideandDestroy _asbp_base_enemy)
  (Variables|/Game/Bluprints/Enemies/UI/BPW_HPBar.BPW_HPBar_C|SetHP (.AsBPW%20HPBar (Utilities|Casting|CastToBPW_HPBar (UserInterface|GetWidget (Variables|Default|GetHealth)))) (/ (Math|Conversions|ToFloat(Integer) (Variables|Default|GetHP)) (Math|Conversions|ToFloat(Integer) (Variables|Default|GetMaxHP))))
  (if (<= (Variables|Default|GetHP) 0)
    (Default|Fadein (.AsBP%20KTWOPGame%20Instance (Utilities|Casting|CastToBP_KTWOPGameInstance (Game|GetGameInstance))) "NewEnumerator2")
    (Utilities|FlowControl|Delay 3.0)
    (Game|OpenLevel(byObjectReference) "/Game/Maps/Levels/L_World.L_World")
    (else
      (CallFunction|EnemyDefeated))))

(event Custom|EnemyDefeated
  (Math|Integer|IncrementInt (Variables|Default|GetEnemiesDefeated)
    (:%20%20
      (if (>= (Variables|Default|GetEnemiesDefeated) (Variables|Default|GetEnemiesCount))
        (bind _asbp_ktwopgame_instance (Utilities|Casting|CastToBP_KTWOPGameInstance (Game|GetGameInstance)))
        (if (Utilities|Enum|Equal(Enum) (Utilities|Array|Get(acopy) (Variables|/Game/Bluprints/Enemies/BP_KTWOPGameInstance.BP_KTWOPGameInstance_C|GetLevelsState _asbp_ktwopgame_instance) (+ (Variables|/Game/Bluprints/Enemies/BP_KTWOPGameInstance.BP_KTWOPGameInstance_C|GetCurrentLevel _asbp_ktwopgame_instance) 1)) "NewEnumerator1")
          (Utilities|Array|SetArrayElem (Variables|/Game/Bluprints/Enemies/BP_KTWOPGameInstance.BP_KTWOPGameInstance_C|GetLevelsState _asbp_ktwopgame_instance) (+ (Variables|/Game/Bluprints/Enemies/BP_KTWOPGameInstance.BP_KTWOPGameInstance_C|GetCurrentLevel _asbp_ktwopgame_instance) 1) "NewEnumerator0"))
        (Utilities|Array|SetArrayElem (Variables|/Game/Bluprints/Enemies/BP_KTWOPGameInstance.BP_KTWOPGameInstance_C|GetLevelsState _asbp_ktwopgame_instance) (Variables|/Game/Bluprints/Enemies/BP_KTWOPGameInstance.BP_KTWOPGameInstance_C|GetCurrentLevel _asbp_ktwopgame_instance) "NewEnumerator2")
        (Default|SaveGame _asbp_ktwopgame_instance)
        (Default|Fadein (.AsBP%20KTWOPGame%20Instance (Utilities|Casting|CastToBP_KTWOPGameInstance (Game|GetGameInstance))) "NewEnumerator1")
        (Utilities|FlowControl|Delay 3.0)
        (Game|OpenLevel(byObjectReference) "/Game/Maps/Levels/L_World.L_World")))))

(event EventBeginPlay
  (bind _health (Variables|Default|GetHealth))
  (bind _returnvalue (UserInterface|GetWidget _health))
  (bind _asbpw_hpbar (Utilities|Casting|CastToBPW_HPBar _returnvalue))
  (Rendering|SetVisibility (Variables|Default|GetWidget) false false)
  (Variables|/Game/Bluprints/Enemies/UI/BPW_HPBar.BPW_HPBar_C|SetHP _asbpw_hpbar 1.0)
  (Variables|/Game/Bluprints/Enemies/UI/BPW_HPBar.BPW_HPBar_C|SetColor _asbpw_hpbar "(R=0.173937,G=1.000000,B=0.000000,A=1.000000)")
  (Variables|Default|SetHP (Variables|Default|GetMaxHP)))

(event Collision|EventActorBeginOverlap
  (params (OtherActor :type Actor%20Object%20Reference)))

(event EventTick
  (params (DeltaSeconds :type Float%20%28single-precision%29)))

(fn ConstructionScript
  (bind _tile (CallFunction|GetUndertile (Transformation|GetActorLocation) 1e+02))
  (Utilities|IsValid _tile
    (:Is%20Valid
      (bind _position (Default|GetSocketPosition _tile))
      (Transformation|SetWorldLocation (Variables|Default|GetPoint) _position false false))))