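; BP_Bear is a bear enemy Blueprint that toggles the visuals for elemental effects.
; The ice switch shows or hides components for the four legs and the body, while plasma and toxic each toggle a single component.
; The lightning switch is an empty stub, BeginPlay and Tick are disabled, and the construction script only calls its parent.
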(event EventBeginPlay
  (|CallParentFunction) ; This node is disabled and will not be called.\nDrag off pins to build functionality.
)

(event EventTick
  (params (DeltaSeconds :type Float%20%28single-precision%29))
  (|CallParentFunction DeltaSeconds) ; This node is disabled and will not be called.\nDrag off pins to build functionality.
)

(event EventSwitchLightning
  (params (IsOn :type Boolean)))

(event EventSwitchIce
  (params (IsOn :type Boolean))
  (for _array_element (Utilities|Array|MakeArray (Variables|Default|GetFrontRightLeg) (Variables|Default|GetFrontLeftLeg) (Variables|Default|GetBackLeftLeg) (Variables|Default|GetBackRightLeg) (Variables|Default|GetBody))
    (Rendering|SetVisibility _array_element IsOn false)))

(event EventSwitchPlasma
  (params (IsOn :type Boolean))
  (Rendering|SetVisibility (Variables|Default|GetPlasma) IsOn false))

(event EventSwitchToxic
  (params (IsOn :type Boolean))
  (Rendering|SetVisibility (Variables|Default|GetToxicFog) IsOn false))

(fn ConstructionScript
  (|CallParentFunction))