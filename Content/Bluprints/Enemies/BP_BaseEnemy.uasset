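; Base enemy Blueprint that handles health display, fade in and out, and death rewards.
; On BeginPlay it creates dynamic material instances, whose Visibility parameter timelines animate to show or hide the mesh.
; Damage updates a widget HP bar, visible only at partial health, and an emissive material's Alpha.
; Death runs once, removing collision, fading out, destroying the actor, adding Stones and Souls to the GameInstance and notifying Aim.
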(event EventBeginPlay
  (bind _asbpw_hpbar (Utilities|Casting|CastToBPW_HPBar (UserInterface|GetWidget (Variables|Default|GetWidget))))
  (Variables|Default|SetHPBar _asbpw_hpbar)
  (Variables|/Game/Bluprints/Enemies/UI/BPW_HPBar.BPW_HPBar_C|SetColor (Variables|Default|GetHPBar) "(R=0.359375,G=0.000000,B=0.000000,A=1.000000)")
  (Widget|SetVisibility (Variables|Default|GetHPBar) "Hidden")
  (CallFunction|MaterialstoMaterialInstances)
  (Variables|Default|SetHealthMaterial (Utilities|Array|Get(acopy) (Variables|Default|GetMaterials) (Variables|Default|GetEmissiveIndex)))
  (bind _visibilitycurve (Timeline|VisibilityTimeline PlayFromStart)
    (:Update
      (CallFunction|SetVisibility _visibilitycurve))))

(event EventHideandDestroy
  (bind _visibilitycurve (Timeline|Timeline_0 PlayFromStart)
    (:Update
      (CallFunction|SetVisibility _visibilitycurve))
    (:Finished
      (Actor|DestroyActor))))

(event EventShowApplyedDamage
  (params (damage :type Float%20%28single-precision%29))
  (Development|PrintString (Utilities|String|ToString(Float) damage)))

(event EventOnDeath
  (bind _returnvalue (Game|GetGameInstance))
  (bind _asbp_ktwopgame_instance (Utilities|Casting|CastToBP_KTWOPGameInstance _returnvalue))
  (Utilities|FlowControl|DoOnce false
    (:Completed
      (Rendering|Material|SetScalarParameterValue (Variables|Default|GetHealthMaterial) "Alpha" 1.0 :!class /Script/Engine.MaterialInstanceDynamic)
      (Components|DestroyComponent (Variables|Default|GetCollisionComponent))
      (bind _visibilitycurve (Timeline|UnvisibilityTimeline PlayFromStart)
        (:Update
          (CallFunction|SetVisibility _visibilitycurve))
        (:Finished
          (Actor|DestroyActor)
          (Class|KTWOPGameInstance|IncreaseStones _asbp_ktwopgame_instance (Variables|Default|Getstone_cost))
          (Class|KTWOPGameInstance|IncreaseSouls _asbp_ktwopgame_instance (Variables|Default|Getsoul_cost))
          (Development|PrintString (Utilities|String|Append "Stones:" (Utilities|String|ToString(Integer) (Variables|/Script/GameplaySystem.KTWOPGameInstance|GetStones _asbp_ktwopgame_instance)) " 
" "Souls: " (Utilities|String|ToString(Integer) (Variables|/Script/GameplaySystem.KTWOPGameInstance|GetSouls _asbp_ktwopgame_instance))))
          (Default|EnemyDefeated (Variables|Default|GetAim)))))))

(event EventDamageApplied
  (params (damage :type Float%20%28single-precision%29) (healthPercent :type Float%20%28single-precision%29))
  (Variables|/Game/Bluprints/Enemies/UI/BPW_HPBar.BPW_HPBar_C|SetHP (Variables|Default|GetHPBar) healthPercent)
  (Rendering|Material|SetScalarParameterValue (Variables|Default|GetHealthMaterial) "Alpha" (- 1.0 healthPercent) :!class /Script/Engine.MaterialInstanceDynamic)
  (if (or (Utilities|IsFull) (Utilities|IsEmpty))
    (Widget|SetVisibility (Variables|Default|GetHPBar) "Hidden")
    (else
      (Widget|SetVisibility (Variables|Default|GetHPBar) "Visible"))))

(fn ConstructionScript)

(fn SetVisibility
  (params (Value :type Float%20%28double-precision%29))
  (for _array_element (Variables|Default|GetMaterials)
    (Rendering|Material|SetScalarParameterValue _array_element "Visibility" Value :!class /Script/Engine.MaterialInstanceDynamic)))

(fn MaterialstoMaterialInstances
  (for (_array_element _array_index) (Rendering|Material|GetMaterials (Variables|Default|GetSkeletalMesh))
    (bind _returnvalue (Rendering|Material|CreateDynamicMaterialInstance _array_element "None" "None" :!class /Script/Engine.KismetMaterialLibrary))
    (Rendering|Material|SetMaterial (Variables|Default|GetSkeletalMesh) _array_index _returnvalue)
    (Utilities|Array|Add (Variables|Default|GetMaterials) _returnvalue)))