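; BP_KTWOPGameInstance is the game instance that holds saved progress and handles screen fades for win, defeat and loading.
; SaveGame and LoadGame copy souls, level states and building levels to and from a BP_SaveGame object in one slot.
; FadeIn stores WINFLAG and shows a win or defeat end screen; its simple-start case only prints a message.
; FadeOut uses that flag to fade a loading screen or the stored end screen.
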(fn SaveGame
  (bind _returnvalue (SaveGame|CreateSaveGameObject "/Game/Bluprints/BP_SaveGame.BP_SaveGame_C"))
  (bind _output_get (LocalVariables|SetSaveObject _returnvalue))
  (Variables|/Game/Bluprints/BP_SaveGame.BP_SaveGame_C|SetSouls _output_get (Variables|Default|GetSouls))
  (Variables|/Game/Bluprints/BP_SaveGame.BP_SaveGame_C|SetLevelsState (LocalVariables|GetSaveObject) (Variables|Default|GetLevelsState))
  (Variables|/Game/Bluprints/BP_SaveGame.BP_SaveGame_C|SetBuildingsLevels (LocalVariables|GetSaveObject) (Variables|Default|GetBuildingsLevels))
  (SaveGame|SaveGametoSlot (LocalVariables|GetSaveObject) "MAIN_SAVE"))

(fn LoadGame
  (bind _returnvalue (SaveGame|LoadGamefromSlot "MAIN_SAVE"))
  (bind _asbp_save_game (Utilities|Casting|CastToBP_SaveGame _returnvalue)
    (:then
      (Variables|Default|SetLevelsState (Variables|/Game/Bluprints/BP_SaveGame.BP_SaveGame_C|GetLevelsState _asbp_save_game))
      (Variables|Default|SetSouls (Variables|/Game/Bluprints/BP_SaveGame.BP_SaveGame_C|GetSouls _asbp_save_game))
      (Variables|Default|SetBuildingsLevels (Variables|/Game/Bluprints/BP_SaveGame.BP_SaveGame_C|GetBuildingsLevels _asbp_save_game)))
    (:CastFailed
      (Development|PrintString "Nothing saved"))))

(fn Fadein
  (params (WINFLAG :type E_WorldStart%20Enum :default "NewEnumerator0"))
  (bind _output_get (Variables|Default|SetWINFLAG WINFLAG))
  (switch Utilities|FlowControl|Switch|SwitchonE_WorldStart _output_get
    (:NewEnumerator0
      (Development|PrintString "Noup, it's doesn't work"))
    (:NewEnumerator1
      (bind _returnvalue (UserInterface|CreateWidget "/Game/UI/UI_Menu/W_EndScreen.W_EndScreen_C" 0 true))
      (Variables|Default|SetGAMEFADE _returnvalue)
      (UserInterface|Viewport|AddtoViewport (Variables|Default|GetGAMEFADE) 0)
      (Rendering|Components|TextRender|SetText (Variables|/Game/UI/UI_Menu/W_EndScreen.W_EndScreen_C|GetText (Variables|Default|GetGAMEFADE)) "Победа")
      (Default|Fadein (Variables|Default|GetGAMEFADE)))
    (:NewEnumerator2
      (bind _returnvalue_2 (UserInterface|CreateWidget "/Game/UI/UI_Menu/W_EndScreen.W_EndScreen_C"))
      (Variables|Default|SetGAMEFADE _returnvalue_2)
      (UserInterface|Viewport|AddtoViewport (Variables|Default|GetGAMEFADE) 0)
      (Rendering|Components|TextRender|SetText (Variables|/Game/UI/UI_Menu/W_EndScreen.W_EndScreen_C|GetText (Variables|Default|GetGAMEFADE)) "Поражение")
      (Default|Fadein (Variables|Default|GetGAMEFADE)))))

(fn FadeOut
  (switch Utilities|FlowControl|Switch|SwitchonE_WorldStart (Variables|Default|GetWINFLAG)
    (:NewEnumerator0
      (bind _returnvalue (UserInterface|CreateWidget "/Game/UI/UI_Menu/W_LoadingScreen.W_LoadingScreen_C"))
      (UserInterface|Viewport|AddtoViewport _returnvalue 0)
      (Default|FadeOut _returnvalue))
    (:NewEnumerator1
      (UserInterface|Viewport|AddtoViewport (Variables|Default|GetGAMEFADE) 0 :!label _label)
      (Default|FadeOut (Variables|Default|GetGAMEFADE))
      (Variables|Default|SetWINFLAG "NewEnumerator0"))
    (:NewEnumerator2
      (goto _label))))