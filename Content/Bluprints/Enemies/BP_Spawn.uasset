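; BP_Spawn is an enemy spawn point that spawns a given list of enemy classes at its Point component.
; Construction places Point on the socket position of the tile beneath the actor.
; BeginPlay hides the widget, waits an initial delay, then sets itself active and colours its particle system red.
; SpawnEnemies runs a delayed loop calling SpawnEnamy, which passes each enemy its Aim and decrements Count; Reset deactivates the spawner.
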(event Custom|Reset
  (Variables|Default|SetIsActive false))

(event Custom|SpawnEnemies
  (params (Enemies :type Array%20of%20BP%20Base%20Enemy%20Class%20References) (Delay :type Float%20%28double-precision%29))
  (bind _index (Utilities|ForwithDelay 0 (- (Utilities|Array|Length Enemies) 1) Delay)
    (:LoopBody
      (CallFunction|SpawnEnamy (Utilities|Array|Get(acopy) Enemies _index)))))

(event EventTick
  (params (DeltaSeconds :type Float%20%28single-precision%29)))

(event EventBeginPlay
  (Rendering|SetVisibility (Variables|Default|GetWidget) false false)
  (Utilities|FlowControl|Delay (Variables|Default|GetInitialDelay))
  (Variables|Default|SetIsActive true)
  (Effects|Components|ParticleSystem|SetVectorParameter (Variables|Default|GetParticleSystem) "Color" (Math|Conversions|ToVector(LinearColor) "(R=100.000000,G=0.151042,B=0.183890,A=0.000000)")))

(fn ConstructionScript
  (bind _tile (CallFunction|GetUndertile (Transformation|GetActorLocation) 1e+02))
  (bind _position (Default|GetSocketPosition _tile))
  (Transformation|SetWorldLocation (Variables|Default|GetPoint) _position false false))

(fn SpawnEnamy
  (params (EnemyType :type BP%20Base%20Enemy%20Class%20Reference))
  (bind _returnvalue (Game|SpawnActorfromClass EnemyType (Math|Transform|MakeTransform (Transformation|GetWorldLocation (Variables|Default|GetPoint))) "AdjustIfPossibleButAlwaysSpawn" 0 0))
  (LocalVariables|SetEnemy _returnvalue)
  (Variables|/Game/Bluprints/Enemies/BP_BaseEnemy.BP_BaseEnemy_C|SetAim (LocalVariables|GetEnemy) (Variables|Default|GetAim))
  (Math|Integer|DecrementInt (Variables|Default|GetCount)))