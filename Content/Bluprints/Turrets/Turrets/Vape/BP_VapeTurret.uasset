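; Vape turret that fires a smoke blast and recolors itself for Lightning, Ice, Toxic and Plasma modes.
; Firing is driven by the anim Blueprint's Shoot dispatcher, which triggers the Blast effect, a random blow sound and RealShoot, while EventShoot is left empty.
; Mode events tint the Blast and Smoke particles plus an emissive dynamic material, and Turnon sizes the blast to the turret's modified radius.
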(event Custom|OnShoot
  (Components|Activation|Activate (Variables|Default|GetBlast) true)
  (Audio|PlaySoundatLocation "/Game/Sounds/Blow/Cues/RandomBlow.RandomBlow" (Transformation|GetActorLocation) "0, 0, 0" 1.0 1.0 0.0 0 0 0 0)
  (Class|Shootable|RealShoot 0.0))

(event EventBeginPlay
  (CallFunction|CreateDMIs)
  (bind _asbpa_vape_turret (Utilities|Casting|CastToBPA_VapeTurret (Components|SkeletalMesh|GetAnimInstance (Variables|Default|GetVape))))
  (EventDispatchers|AssignShoot _asbpa_vape_turret (delegate Custom|OnShoot)))

(event EventLightningon
  (CallFunction|ChangeSmokeColor "(R=0.000000,G=0.000000,B=1.000000,A=1.000000)")
  (CallFunction|SetColor "(R=0.000000,G=0.000000,B=1.000000,A=1.000000)"))

(event EventIceon
  (CallFunction|ChangeSmokeColor "(R=0.200000,G=0.600000,B=1.000000,A=1.000000)")
  (CallFunction|SetColor "(R=0.000000,G=0.600000,B=1.000000,A=1.000000)"))

(event EventEventShoot
  (params (DeltaTime :type Float%20%28single-precision%29)))

(event EventToxicon
  (CallFunction|ChangeSmokeColor "(R=0.200000,G=1.000000,B=0.200000,A=1.000000)")
  (CallFunction|SetColor "(R=0.000000,G=1.000000,B=0.000000,A=1.000000)"))

(event EventPlasmaon
  (CallFunction|ChangeSmokeColor "(R=1.000000,G=0.400000,B=1.000000,A=1.000000)")
  (CallFunction|SetColor "(R=1.000000,G=0.000000,B=1.000000,A=1.000000)"))

(event EventTurnon
  (Niagara|SetNiagaraVariable(Float) (Variables|Default|GetBlast) "User.Size" (.turretradius (Variables|Default|GetModifiedStats))))

(fn ConstructionScript)

(fn ChangeSmokeColor
  (params (Color :type Linear%20Color%20Structure))
  (Effects|Components|ParticleSystem|SetColorParameter (Variables|Default|GetBlast) "User.Color" Color)
  (Effects|Components|ParticleSystem|SetColorParameter (Variables|Default|GetSmoke) "User.Color" Color))

(fn CreateDMIs
  (bind _returnvalue (Rendering|Material|CreateDynamicMaterialInstance (Variables|Default|GetVape) 1 "/Game/Bluprints/Turrets/Materials/MI_EmmissiveTurret.MI_EmmissiveTurret" "None" :!class /Script/Engine.PrimitiveComponent))
  (Variables|Default|SetDMI _returnvalue))

(fn SetColor
  (params (NewParam :type Linear%20Color%20Structure))
  (Rendering|Material|SetVectorParameterValue (Variables|Default|GetDMI) "Color" NewParam :!class /Script/Engine.MaterialInstanceDynamic))