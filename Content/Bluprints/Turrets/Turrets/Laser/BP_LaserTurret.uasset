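; Laser turret Blueprint that passes its shoot event to RealShoot and recolors its emissive parts by elemental type.
; On BeginPlay it creates dynamic instances of the emissive turret material on two mesh slots and stores them in an array.
; Lightning, Ice, Toxic and Plasma events each call SetColor, which writes that element's color to the Color parameter of every stored instance.
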(event EventBeginPlay
  (CallFunction|CreateDMIs))

(event EventEventShoot
  (params (DeltaTime :type Float%20%28single-precision%29))
  (Class|Shootable|RealShoot DeltaTime))

(event EventLightningon
  (CallFunction|SetColor "(R=0.000000,G=0.000000,B=1.000000,A=1.000000)"))

(event EventIceon
  (CallFunction|SetColor "(R=0.000000,G=0.600000,B=1.000000,A=1.000000)"))

(event EventToxicon
  (CallFunction|SetColor "(R=0.000000,G=1.000000,B=0.000000,A=1.000000)"))

(event EventPlasmaon
  (CallFunction|SetColor "(R=1.000000,G=0.000000,B=1.000000,A=1.000000)"))

(fn ConstructionScript)

(fn CreateDMIs
  (bind _returnvalue (Rendering|Material|CreateDynamicMaterialInstance (Variables|Default|GetMesh) 1 "/Game/Bluprints/Turrets/Materials/MI_EmmissiveTurret.MI_EmmissiveTurret" "None" :!class /Script/Engine.PrimitiveComponent))
  (Utilities|Array|Add (Variables|Default|GetDMIs) _returnvalue)
  (bind _returnvalue_2 (Rendering|Material|CreateDynamicMaterialInstance (Variables|Default|GetMesh) 4 "/Game/Bluprints/Turrets/Materials/MI_EmmissiveTurret.MI_EmmissiveTurret" "None" :!class /Script/Engine.PrimitiveComponent))
  (Utilities|Array|Add (Variables|Default|GetDMIs) _returnvalue_2))

(fn SetColor
  (params (Color :type Linear%20Color%20Structure))
  (for _array_element (Variables|Default|GetDMIs)
    (Rendering|Material|SetVectorParameterValue _array_element "Color" Color :!class /Script/Engine.MaterialInstanceDynamic)))